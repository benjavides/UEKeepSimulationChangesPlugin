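; BP_KeepActorSimulationChanges is a utility Blueprint that keeps changes made to an actor during simulation.
; On BeginPlay it enables player 0 input if a SaveKey is set, then calls KeepActorSimulatedChanges on the Actor reference when that key is pressed.
; A custom event taking an EndPlayReason makes the same call on the Blueprint itself, not that reference, when SaveAtEndPlay is enabled.
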(event Custom|CustomEvent
  (params (EndPlayReason :type EEndPlayReason%20Enum :default "Destroyed"))
  (if (Variables|Default|GetSaveAtEndPlay)
    (Class|KeepSimulationChangesBPLibrary|KeepActorSimulatedChanges self)))

(event EventBeginPlay
  (if (not (== (Variables|Default|GetSaveKey) "None"))
    (Input|EnableInput (Game|GetPlayerController 0))))

(event Input|KeyboardEvents|AnyKey
  (params (Key :type Key%20Structure :default "None"))
  (:Pressed
    (if (== Key (Variables|Default|GetSaveKey))
      (Class|KeepSimulationChangesBPLibrary|KeepActorSimulatedChanges (Variables|Default|GetActor)))))

(fn ConstructionScript)